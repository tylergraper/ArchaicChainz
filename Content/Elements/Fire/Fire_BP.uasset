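; Fire_BP is a fire actor with a flickering point light that turns to face the player's camera.
; On BeginPlay, a LightFlicker timeline scales the point light's intensity by its Flicker track.
; A looping timer calls GetAngle, which yaws the whole actor toward the camera on the horizontal plane, billboard-style, at short intervals rather than every tick.
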(event `self.ReceiveBeginPlay`
  (`KismetSystemLibrary.K2_SetTimer` null "GetAngle" 0.1 true)
  (bind (_direction _flicker) (`Timeline|Light Flicker`)
    (:`Update`
      (`LightComponent.SetIntensity` (`self.PointLight`) (* (`self.Light  Intensity`) _flicker)))))

(fn `GetAngle`
  (`self.K2_SetActorRotation` (`KismetMathLibrary.Conv_VectorToRotator` (`KismetMathLibrary.Normal` (* (- (`PlayerCameraManager.GetCameraLocation` (`GameplayStatics.GetPlayerCameraManager` 0)) (`self.K2_GetActorLocation`)) (1.0 1.0 0.0))))))

(fn `UserConstructionScript`)