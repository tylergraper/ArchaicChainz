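; Grappling hook projectile actor that flies out, returns to its spawn point and drags a hit jack along with it.
; BeginPlay stores the sphere's start location, then after a short delay the Comeback timeline zeroes projectile velocity and lerps the sphere back.
; A hit also triggers Comeback, and a second timeline lerps a hit jack's capsule to the start point.
; Either timeline destroys the hook when it finishes.
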(event `self.ReceiveBeginPlay`
  (bind _returnvalue (`SceneComponent.K2_GetComponentLocation` (`self.Sphere`)))
  (bind _output_get (set `self.location` _returnvalue))
  (`KismetSystemLibrary.Delay` 0.2)
  (bind (_direction _newtrack_0) (`Timeline|comeback` :!label _label)
    (:`Update`
      (set `MovementComponent.Velocity` (0.0 0.0 0.0) (`self.ProjectileMovement`))
      (`SceneComponent.K2_SetWorldLocation` (`self.Sphere`) (`KismetMathLibrary.VLerp` _returnvalue _output_get _newtrack_0) false false))
    (:`Finished`
      (`self.K2_DestroyActor`))))

(event `self.Sphere.OnComponentHit`
  (params (HitComponent :type "PrimitiveComponent Object Reference") (OtherActor :type "Actor Object Reference") (OtherComp :type "PrimitiveComponent Object Reference") (NormalImpulse :type "Vector Structure") (Hit :type "HitResult Structure (by ref)"))
  (`|ExecutionSequence`
    (:`then_0`
      (goto _label))
    (:`then_1`
      (bind _asjack (cast `/Game/bp_hook/jack` OtherActor))
      (bind (_direction _newtrack_0) (`Timeline|Timeline_0`)
        (:`Update`
          (bind _capsule (`/Game/bp_hook/jack.Capsule` _asjack))
          (`SceneComponent.K2_SetWorldLocation` _capsule (`KismetMathLibrary.VLerp` (`SceneComponent.K2_GetComponentLocation` _capsule) (`self.location`) _newtrack_0) false false))
        (:`Finished`
          (`self.K2_DestroyActor`))))))

(fn `UserConstructionScript`)